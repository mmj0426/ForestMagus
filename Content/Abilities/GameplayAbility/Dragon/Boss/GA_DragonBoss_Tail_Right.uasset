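; Gameplay ability for the dragon boss's right tail attack, inferred from its name, built on a montage and tail collision.
; After committing, it sets the boss's TailCollision to overlap pawns and plays the montage, ending on blend-out, interrupt or cancel.
; Montage events only build an effect container spec, without applying it here.
; On end, it stops the task and has a NoCollision reset behind a seemingly inverted reference check.
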(event `self.K2_ActivateAbility`
  (bind _returnvalue_owneractor (break `GameplayAbilityActorInfo` (`self.GetActorInfo`)))
  ;[1 1 1] 어빌리티 실행 시도
  (bind _returnvalue (`self.K2_CommitAbility`)) ; 설정한 조건에 따라서 실패할수도있음 (예를 들어 마나가 없거나 특정 애니메이션이 실행중일때)
  (if _returnvalue
    (`|ExecutionSequence`
      (:`then_0`
        (bind _asbp_dragon_boss (cast `/Game/Characters/Elemental_Dragon/Dragon/BP_Dragon_Boss` _returnvalue_owneractor))
        (set `self.BP Dragon Boss` _asbp_dragon_boss)
        (`PrimitiveComponent.SetCollisionProfileName` (`/Game/Characters/Elemental_Dragon/Dragon/BP_Dragon_Boss.TailCollision` _asbp_dragon_boss) "OverlapOnlyPawn" true))
      (:`then_1`
        (bind (_asynctaskproxy _eventtag _eventdata) (`ATask_PlayMontageAndWaitForEvent.PlayMontageAndWaitForEvent` "None" (`self.MontageToPlay`))
          (:`then`
            (set `self.Async Task` _asynctaskproxy))
          (:`OnBlendOut`
            (`self.K2_EndAbility` :!label _label))
          (:`OnInterrupted`
            (goto _label))
          (:`OnCancelled`
            (goto _label))
          (:`EventReceived`
            (`self.MakeEffectContainerSpec` _eventtag _eventdata)))))))

(event `self.K2_OnEndAbility`
  (params (bWasCancelled :type Boolean))
  (bind _bp_dragon_boss (`self.BP Dragon Boss`))
  (bind _async_task (`self.Async Task`))
  (if (not (!= _bp_dragon_boss null))
    (`PrimitiveComponent.SetCollisionProfileName` (`/Game/Characters/Elemental_Dragon/Dragon/BP_Dragon_Boss.TailCollision` _bp_dragon_boss) "NoCollision" true))
  (`/Engine/EditorBlueprintResources/StandardMacros.IsValid` _async_task
    (:`Is Valid`
      (`GameplayTask.EndTask` _async_task)
      (`parent.K2_OnEndAbility` bWasCancelled))))