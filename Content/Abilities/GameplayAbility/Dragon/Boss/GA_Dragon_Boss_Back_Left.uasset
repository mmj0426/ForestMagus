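; Gameplay ability for the dragon boss, named for a back-left action.
; On activation it runs the parent logic, then snaps the owning boss's yaw by a small fixed positive step.
; GetSpawnTransform builds a transform at the mesh's head socket, nudged along the capsule's forward vector and using the capsule's rotation; this graph never calls it.
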(event `self.K2_ActivateAbility`
  (bind _returnvalue_owneractor (break `GameplayAbilityActorInfo` (`self.GetActorInfo`)))
  (`parent.K2_ActivateAbility`)
  (bind _asbp_dragon_boss (cast `/Game/Characters/Elemental_Dragon/Dragon/BP_Dragon_Boss` _returnvalue_owneractor))
  (bind (_returnvalue_roll _returnvalue_pitch _returnvalue_yaw) (`KismetMathLibrary.BreakRotator` (`Actor.K2_GetActorRotation` _asbp_dragon_boss)))
  (`Actor.K2_SetActorRotation` _asbp_dragon_boss (`KismetMathLibrary.MakeRotator` _returnvalue_roll _returnvalue_pitch (+ _returnvalue_yaw 10.0)) false))

(fn `GetSpawnTransform`
  (returns (Result :type "Transform Structure"))
  (bind _returnvalue_owneractor (break `GameplayAbilityActorInfo` (`self.GetActorInfo`)))
  (bind _asbp_dragon_boss (cast `/Game/Characters/Elemental_Dragon/Dragon/BP_Dragon_Boss` _returnvalue_owneractor))
  (bind _capsulecomponent (`Character.CapsuleComponent` _asbp_dragon_boss))
  (bind _output_get (set `self.SpawnTransform` (`KismetMathLibrary.MakeTransform` (+ (`SceneComponent.GetSocketLocation` (`Character.Mesh` _asbp_dragon_boss) "HeadSocket") (`SceneComponent.GetForwardVector` _capsulecomponent)) (`SceneComponent.K2_GetComponentRotation` _capsulecomponent))))
  (return _output_get))