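; GA_Dragon_Tail_Right is a GAS gameplay ability for the dragon, by its name a right tail attack, driven by a montage.
; After a successful commit it plays the montage and turns each received gameplay event into an effect container spec, then applies it.
; Blend out, interruption or cancellation ends the ability.
; On end, a still-valid montage task is stopped, and only then is the parent end handler called.
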(event `self.K2_ActivateAbility`
  ;[1 1 1] 어빌리티 실행 시도
  (bind _returnvalue (`self.K2_CommitAbility`)) ; 설정한 조건에 따라서 실패할수도있음 (예를 들어 마나가 없거나 특정 애니메이션이 실행중일때)
  (if _returnvalue
    (bind (_asynctaskproxy _eventtag _eventdata) (`ATask_PlayMontageAndWaitForEvent.PlayMontageAndWaitForEvent` "None" (`self.MontageToPlay`))
      (:`then`
        (set `self.Async Task` _asynctaskproxy))
      (:`OnBlendOut`
        (`self.K2_EndAbility` :!label _label))
      (:`OnInterrupted`
        (goto _label))
      (:`OnCancelled`
        (goto _label))
      (:`EventReceived`
        (bind _returnvalue_2 (`self.MakeEffectContainerSpec` _eventtag _eventdata))
        (bind _returnvalue_3 (`FMBlueprintLibrary.AddTargetsToEffectContainerSpec` _returnvalue_2))
        (`FMBlueprintLibrary.ApplyExternalEffectContainerSpec` _returnvalue_3)))))

(event `self.K2_OnEndAbility`
  (params (bWasCancelled :type Boolean))
  (bind _async_task (`self.Async Task`))
  (`/Engine/EditorBlueprintResources/StandardMacros.IsValid` _async_task
    (:`Is Valid`
      (`GameplayTask.EndTask` _async_task)
      (`parent.K2_OnEndAbility` bWasCancelled))))