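; GA_DragonRed_RedFireBall is the red dragon's fireball gameplay ability, with activation deferred entirely to its parent class.
; GetSpawnTransform casts the owner actor to BP_Dragon_Red and builds a unit-scale transform from the HeadSocket location plus the capsule's forward vector.
; The transform takes the capsule's world rotation, so its orientation follows the body instead of the head socket.
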(event `self.K2_ActivateAbility`
  (`parent.K2_ActivateAbility`))

(fn `GetSpawnTransform`
  (returns (Result :type "Transform Structure"))
  (bind _returnvalue_owneractor (break `GameplayAbilityActorInfo` (`self.GetActorInfo`)))
  (bind _asbp_dragon_red (cast `/Game/Characters/Elemental_Dragon/Dragon/BP_Dragon_Red` _returnvalue_owneractor))
  (bind _capsulecomponent (`Character.CapsuleComponent` _asbp_dragon_red))
  (bind _output_get (set `self.SpawnTransform` (`KismetMathLibrary.MakeTransform` (+ (`SceneComponent.GetSocketLocation` (`Character.Mesh` _asbp_dragon_red) "HeadSocket") (`SceneComponent.GetForwardVector` _capsulecomponent)) (`SceneComponent.K2_GetComponentRotation` _capsulecomponent))))
  (return _output_get))