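; GA_DragonRed_WaterFireBall is a red dragon gameplay ability, by its name a water fireball attack.
; Activation and end events only call the parent, which holds the ability logic.
; GetSpawnTransform builds a transform at the dragon mesh's HeadSocket plus the capsule's unit forward vector, using capsule rotation and unit scale.
; A 500-unit scaling of that forward vector is left unconnected.
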(event `self.K2_ActivateAbility`
  (`parent.K2_ActivateAbility`))

(event `self.K2_OnEndAbility`
  (params (bWasCancelled :type Boolean))
  (`parent.K2_OnEndAbility` bWasCancelled))

(fn `GetSpawnTransform`
  (returns (Result :type "Transform Structure"))
  (bind _returnvalue_owneractor (break `GameplayAbilityActorInfo` (`self.GetActorInfo`)))
  (bind _asbp_dragon_red (cast `/Game/Characters/Elemental_Dragon/Dragon/BP_Dragon_Red` _returnvalue_owneractor))
  (bind _capsulecomponent (`Character.CapsuleComponent` _asbp_dragon_red))
  (bind _output_get (set `self.SpawnTransform` (`KismetMathLibrary.MakeTransform` (+ (`SceneComponent.GetSocketLocation` (`Character.Mesh` _asbp_dragon_red) "HeadSocket") (`SceneComponent.GetForwardVector` _capsulecomponent)) (`SceneComponent.K2_GetComponentRotation` _capsulecomponent))))
  (return _output_get))