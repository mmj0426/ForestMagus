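; GA_FireBall is the player's fireball skill Gameplay Ability, which sets up aim and spawn transform before handing off to its parent's activation.
; A complex line trace from the player camera finds the aim point, and the character turns in yaw to face it.
; SpawnTransform combines the staff's ProjectileSpawn socket location with that yaw-only rotation, so it carries no vertical aim.
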(event `self.K2_ActivateAbility`
  (bind _returnvalue_owneractor (break `GameplayAbilityActorInfo` (`self.GetActorInfo`)))
  (bind _asbp_player_character (cast `/Game/Characters/PlayerCharacter/BP_PlayerCharacter` _returnvalue_owneractor))
  (bind _camera (`PlayerCharacter.Camera` _asbp_player_character))
  (bind _returnvalue (`SceneComponent.K2_GetComponentLocation` _camera))
  (bind _outhit (`KismetSystemLibrary.LineTraceSingleForObjects` _returnvalue (+ _returnvalue (* (`KismetMathLibrary.GetForwardVector` (`SceneComponent.K2_GetComponentRotation` _camera)) 5000.0)) (`|MakeArray` "ObjectTypeQuery1" "ObjectTypeQuery2" "ObjectTypeQuery3" "ObjectTypeQuery4" "ObjectTypeQuery5" "ObjectTypeQuery6" :!type "EObjectTypeQuery Enum") true (`|MakeArray` _asbp_player_character :!type "Actor Object Reference")))
  (bind (_returnvalue_roll _returnvalue_pitch _returnvalue_yaw) (`KismetMathLibrary.BreakRotator` (`KismetMathLibrary.FindLookAtRotation` (`Actor.K2_GetActorLocation` _asbp_player_character) (`.Location` (`GameplayStatics.BreakHitResult` _outhit)))))
  (`Actor.K2_SetActorRotation` _asbp_player_character (`KismetMathLibrary.MakeRotator` 0.0 0.0 _returnvalue_yaw) false)
  (set `self.SpawnTransform` (`KismetMathLibrary.MakeTransform` (`SceneComponent.GetSocketLocation` (`PlayerCharacter.StaffMesh` _asbp_player_character) "ProjectileSpawn") (`KismetMathLibrary.MakeRotator` 0.0 0.0 _returnvalue_yaw)))
  (`parent.K2_ActivateAbility`))