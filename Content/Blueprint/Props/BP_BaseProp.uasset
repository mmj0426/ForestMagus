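; Base prop that reacts to damage by getting knocked away and revealing a field fragment pickup.
; On BeginPlay it pre-spawns a randomized BP_FieldFragment just above the mesh, hidden and without collision.
; OnDamaged pushes the mesh with a fixed force, reveals the fragment with pawn-only overlap, disables capsule collision and destroys the prop after a short delay.
; The IsDamaged flag only limits the debug print to the first hit.
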(event `self.ReceiveBeginPlay`
  (bind (_returnvalue_x _returnvalue_y _returnvalue_z) (`KismetMathLibrary.BreakVector` (`SceneComponent.K2_GetComponentLocation` (`self.PropMesh`))))
  (bind _returnvalue (`|SpawnActorFromClass` :`Class` "/Game/Blueprint/SkillFragment/BP_FieldFragment.BP_FieldFragment_C" :`SpawnTransform` (`KismetMathLibrary.MakeTransform` (`KismetMathLibrary.MakeVector` _returnvalue_x _returnvalue_y (+ _returnvalue_z 60.0))) :`CollisionHandlingOverride` "Undefined" :`TransformScaleMethod` "OverrideRootScale" :`bRandom` true :`Instigator` null))
  (bind _output_get (set `self.Fragment` _returnvalue))
  (`PrimitiveComponent.SetCollisionProfileName` (`BaseSkillFragment.SphereCollision` _output_get) "NoCollision" true)
  (`self.SetActorHiddenInGame` _output_get true))

(event `self.OnDamaged`
  (params (DamageAmount :type "Float (single-precision)") (HitInfo :type "HitResult Structure (by ref)") (DamageTags :type "GameplayTagContainer Structure (by ref)") (InstigatorCharacter :type "BaseCharacter Object Reference") (DamageCauser :type "Actor Object Reference"))
  (bind _propmesh (`self.PropMesh`))
  (bind _fragment (`self.Fragment`))
  (`|ExecutionSequence`
    (:`then_0`
      (if (not (`self.bIsDamaged`))
        (set `self.bIsDamaged` true)
        (`KismetSystemLibrary.PrintString` (`KismetStringLibrary.Concat_StrStr` "On Dmaaged Amount: " (`KismetStringLibrary.Conv_DoubleToString` DamageAmount)) true true (struct :`B` 1.0 :`A` 1.0))))
    (:`then_1`
      (`PrimitiveComponent.AddForceAtLocation` _propmesh (100000.0 100000.0 100000.0) (`SceneComponent.K2_GetComponentLocation` _propmesh) "None")
      (`self.SetActorHiddenInGame` _fragment false)
      (`PrimitiveComponent.SetCollisionProfileName` (`BaseSkillFragment.SphereCollision` _fragment) "OverlapOnlyPawn" true)
      (`PrimitiveComponent.SetCollisionProfileName` (`self.CapsuleComponent`) "NoCollision" true)
      (`KismetSystemLibrary.Delay` 2.0)
      (`self.K2_DestroyActor`))))

(fn `UserConstructionScript`)