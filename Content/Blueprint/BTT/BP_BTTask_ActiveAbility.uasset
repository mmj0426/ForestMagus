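; Behavior Tree task that makes a BaseMonster pawn activate a skill ability and waits until it ends.
; It reinitializes probabilities, then activates either an ability chosen by ActivateAbility when IsRandom is set, or the fixed SkillAbility.
; It binds to the end of the first active GA_SkillBase matching AbilityTags and finishes successfully then.
; Failed casts leave the task unfinished.
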(event `self.ReceiveExecuteAI`
  (params (OwnerController :type "AIController Object Reference") (ControlledPawn :type "Pawn Object Reference"))
  (`self.ReInitializeProbability`)
  (bind _asbase_monster (cast `BaseMonster` ControlledPawn))
  (if (`self.bIsRandom`)
    (bind _returnvalue (`self.ActivateAbility`))
    (`BaseMonster.ActiveAbility` _asbase_monster _returnvalue)
    (else
      (`BaseMonster.ActiveAbility` _asbase_monster (`self.SkillAbility`))))
  (bind _activeabilities (`BaseCharacter.GetActiveAbilitiesWithTags` _asbase_monster (`self.AbilityTags`)))
  (bind _asga_skill_base (cast `/Game/Abilities/GameplayAbility/Shared/GA_SkillBase` (`|GetArrayItem` _activeabilities)))
  (add `/Game/Abilities/GameplayAbility/Shared/GA_SkillBase.EndAbility` _asga_skill_base (delegate `EndAbility`)))

(event `EndAbility`
  (`self.FinishExecute` true))