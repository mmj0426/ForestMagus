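; BP_FieldFragment is a skill fragment actor that sets itself up from a data table on BeginPlay.
; If Random is set, it rolls FragmentClassID from the table's row count, assuming rows named by sequential numbers.
; A nonzero ID looks up DT_FragmentClass, copies the SkillAbility and async-loads the mesh and icon.
; Overlap and Tick are empty, and an alternative pick from RandomFragments is left unconnected.
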(event `self.ReceiveBeginPlay`
  (bind _fragmentclassid (`self.FragmentClassID`))
  (if (`self.bRandom`)
    (bind _outrownames (`DataTableFunctionLibrary.GetDataTableRowNames` (`self.Data Table`)))
    (for (_ _array_index) _outrownames
      _)
    (set `self.FragmentClassID` (`KismetMathLibrary.RandomIntegerInRange` 1 (+ _array_index 1))))
  (if (!= _fragmentclassid 0)
    (bind _returnvalue (`|GetDataTableRow` "/Game/Blueprint/SkillFragment/DT_FragmentClass.DT_FragmentClass" (`KismetStringLibrary.Conv_StringToName` (`KismetStringLibrary.Conv_IntToString` _fragmentclassid)))
      (:`then`
        (`|ExecutionSequence`
          (:`then_0`
            (set `self.SkillAbility` (`.SkillAbility_32_B88848EF44AD52CAD7BE40B78FDEC245` (break `/Game/Blueprint/SkillFragment/FragmentClass` _returnvalue))))
          (:`then_1`
            (bind _object (`|LoadAsset` (`.StaticMesh_34_BDB2353D490F610A47DCB58244D4FA31` (break `/Game/Blueprint/SkillFragment/FragmentClass` _returnvalue)))
              (:`Completed`
                (bind _asstatic_mesh (cast `StaticMesh` _object))
                (`StaticMeshComponent.SetStaticMesh` (`self.SkillFragmentMesh`) _asstatic_mesh))))
          (:`then_2`
            (bind _object_2 (`|LoadAsset` (`.SkillIcon_41_E587562C4CC907FD1476BE94298BD415` (break `/Game/Blueprint/SkillFragment/FragmentClass` _returnvalue)))
              (:`Completed`
                (bind _astexture_2d (cast `Texture2D` _object_2))
                (set `self.SkillIcon` _astexture_2d)))))))))

(fn `UserConstructionScript`)