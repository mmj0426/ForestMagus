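; BP_ProjectileBase is a projectile base Blueprint that delivers a gameplay effect container to the actors it overlaps.
; On overlap it records each actor in HitActors so none is hit twice, and skips applying effects to its Instigator.
; For any other new actor, it adds that actor as a target to its EffectContainerSpec and applies the spec as an external effect container.
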(event `self.ReceiveActorBeginOverlap`
  (params (OtherActor :type "Actor Object Reference"))
  (if (not (`KismetArrayLibrary.Array_Contains` (`self.HitActors`) OtherActor))
    (`KismetArrayLibrary.Array_Add` (`self.HitActors`) OtherActor)
    (if (!= OtherActor (`self.GetInstigator`))
      (bind _returnvalue (`FMBlueprintLibrary.AddTargetsToEffectContainerSpec` :`ContainerSpec` (`self.EffectContainerSpec`) :`TargetActors` (`|MakeArray` OtherActor)))
      (`FMBlueprintLibrary.ApplyExternalEffectContainerSpec` _returnvalue))))

(fn `UserConstructionScript`)