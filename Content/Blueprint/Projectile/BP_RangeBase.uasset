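; BP_RangeBase is a base actor for area attacks that deal damage through Gameplay Ability System effect containers.
; ApplyDamageWithTrace runs a multi-sphere object trace from a local-space offset to a point ahead of the actor along its forward vector.
; The hits become targets on the EffectContainerSpec, which is then applied externally.
; Its event graph and construction script are empty, and nothing here calls the damage function.
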(event `self.ReceiveActorBeginOverlap`
  (params (OtherActor :type "Actor Object Reference")))

(event `self.ReceiveDestroyed`)

(fn `Apply Damage With Trace`
  (bind _outhits (`KismetSystemLibrary.SphereTraceMultiForObjects` :`Start` (`KismetMathLibrary.TransformLocation` (`self.GetTransform`) (`self.OffsetFromActor`)) :`End` (+ (* (`self.GetActorForwardVector`) (`self.TraceLength`)) (`self.K2_GetActorLocation`)) :`Radius` (`self.SphereRadius`) :`ObjectTypes` (`self.ObjectTypes`) :`DrawDebugType` (`self.DrawDebug`)))
  (bind _returnvalue (`FMBlueprintLibrary.AddTargetsToEffectContainerSpec` (`self.EffectContainerSpec`) _outhits))
  (`FMBlueprintLibrary.ApplyExternalEffectContainerSpec` _returnvalue))

(fn `UserConstructionScript`)