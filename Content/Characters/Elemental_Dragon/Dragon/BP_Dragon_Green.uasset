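; Green elemental dragon monster Blueprint that keeps a widget-component HP bar in sync with its health.
; On BeginPlay it casts the HPBarWidget's widget to UMG_Monster_HP, caches it and sets the initial bar percent.
; OnHealthChanged refreshes the bar from GetHPPercent and prints the delta and current HP for debugging.
; Overlap, Tick and the construction script are empty.
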(event `self.ReceiveBeginPlay`
  (bind _asumg_monster_hp (cast `/Game/Blueprint/Widget/UMG_Monster_HP` (`WidgetComponent.GetWidget` (`self.HPBar_Widget`))))
  (bind _output_get (set `self.HPWidget` _asumg_monster_hp))
  (bind _returnvalue (`self.GetHP_Percent`))
  (`ProgressBar.SetPercent` (`/Game/Blueprint/Widget/UMG_Monster_HP.HP_Bar` _output_get) _returnvalue))

(event `self.OnHealthChanged`
  (params (DeltaValue :type "Float (single-precision)") (EventTags :type "GameplayTagContainer Structure (by ref)"))
  (bind _returnvalue (`self.GetHP_Percent`))
  (`ProgressBar.SetPercent` (`/Game/Blueprint/Widget/UMG_Monster_HP.HP_Bar` (`self.HPWidget`)) _returnvalue)
  (`KismetSystemLibrary.PrintString` (`KismetStringLibrary.Concat_StrStr` "Call On Health Changed Delta Value: " (`KismetStringLibrary.Conv_DoubleToString` DeltaValue)) true true (struct :`R` 1.0 :`A` 1.0))
  (`KismetSystemLibrary.PrintString` (`KismetStringLibrary.Concat_StrStr` "Current HP: " (`KismetStringLibrary.Conv_DoubleToString` (`self.GetHealth`))) true true (struct :`R` 1.0 :`A` 1.0)))

(fn `UserConstructionScript`)