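; Dragon character Blueprint in the Elemental_Dragon set, built on Gameplay Ability System members and currently holding only debug feedback for health events.
; OnDamaged prints the damage amount, while OnHealthChanged prints the delta and the current HP from GetHealth.
; A disconnected loop that would activate each DefaultAbilities class through the AbilitySystemComponent never runs.
; BeginPlay, overlap, Tick and the construction script are empty.
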(event `self.ReceiveBeginPlay`)

(event `self.OnDamaged`
  (params (DamageAmount :type "Float (single-precision)") (HitInfo :type "HitResult Structure (by ref)") (DamageTags :type "GameplayTagContainer Structure (by ref)") (InstigatorCharacter :type "BaseCharacter Object Reference") (DamageCauser :type "Actor Object Reference"))
  (`KismetSystemLibrary.PrintString` (`KismetStringLibrary.Concat_StrStr` "On Dmaaged Amount: " (`KismetStringLibrary.Conv_DoubleToString` DamageAmount)) true true (struct :`B` 1.0 :`A` 1.0)))

(event `self.OnHealthChanged`
  (params (DeltaValue :type "Float (single-precision)") (EventTags :type "GameplayTagContainer Structure (by ref)"))
  (`KismetSystemLibrary.PrintString` (`KismetStringLibrary.Concat_StrStr` "Call On Health Changed Delta Value: " (`KismetStringLibrary.Conv_DoubleToString` DeltaValue)) true true (struct :`R` 1.0 :`A` 1.0))
  (`KismetSystemLibrary.PrintString` (`KismetStringLibrary.Concat_StrStr` "Current HP: " (`KismetStringLibrary.Conv_DoubleToString` (`self.GetHealth`))) true true (struct :`R` 1.0 :`A` 1.0)))

(fn `UserConstructionScript`)