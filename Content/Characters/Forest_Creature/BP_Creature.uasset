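; BP_Creature is a forest creature NPC that offers dialogue to the player.
; On BeginPlay it spawns a Dialogue_AIController, loops an idle animation, and creates a hidden interaction widget.
; When the player enters DetectCollision, it shows the widget and hands the player its AI controller and BT_Dialogue behavior tree.
; Leaving the area only hides the widget; the player keeps both references.
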(event `self.ReceiveBeginPlay`
  (`|ExecutionSequence`
    (:`then_0`
      (bind _returnvalue (`|SpawnActorFromClass` "/Game/Characters/Forest_Creature/Dialogue_AIController.Dialogue_AIController_C" (`KismetMathLibrary.MakeTransform` (0.0 0.0 0.0)) "Undefined" "OverrideRootScale" null null))
      (set `self.AIController` _returnvalue)
      (`SkeletalMeshComponent.PlayAnimation` (`self.Mesh`) "/Game/Animations/Forest_Creature/Standart/Anim_Idle.Anim_Idle" true))
    (:`then_1`
      (bind _returnvalue_2 (`|CreateWidget` "/Game/Blueprint/Widget/UMG_Interaction.UMG_Interaction_C" (`GameplayStatics.GetPlayerController` 0)))
      (bind _output_get (set `self.InteractionWidget` _returnvalue_2))
      (`UserWidget.AddToViewport` _output_get 0)
      (`Widget.SetVisibility` _output_get "Hidden"))))

(event `self.DetectCollision.OnComponentBeginOverlap`
  (params (OverlappedComponent :type "PrimitiveComponent Object Reference") (OtherActor :type "Actor Object Reference") (OtherComp :type "PrimitiveComponent Object Reference") (OtherBodyIndex :type Integer) (bFromSweep :type Boolean) (SweepResult :type "HitResult Structure (by ref)"))
  (bind _asbp_player_character (cast `/Game/Characters/PlayerCharacter/BP_PlayerCharacter` OtherActor))
  (set `/Game/Characters/PlayerCharacter/BP_PlayerCharacter.AIController` (`self.AIController`) _asbp_player_character)
  (`Widget.SetVisibility` (`self.InteractionWidget`) "Visible")
  (set `/Game/Characters/PlayerCharacter/BP_PlayerCharacter.DialogueTree` "/Game/BehaviorTree/Dialogue/BT_Dialogue.BT_Dialogue" _asbp_player_character))

(event `self.DetectCollision.OnComponentEndOverlap`
  (params (OverlappedComponent :type "PrimitiveComponent Object Reference") (OtherActor :type "Actor Object Reference") (OtherComp :type "PrimitiveComponent Object Reference") (OtherBodyIndex :type Integer))
  (cast `/Game/Characters/PlayerCharacter/BP_PlayerCharacter` OtherActor)
  (`Widget.SetVisibility` (`self.InteractionWidget`) "Hidden"))

(fn `UserConstructionScript`)